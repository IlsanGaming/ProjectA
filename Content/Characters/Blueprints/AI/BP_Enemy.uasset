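; BP_Enemy is an AI enemy character with health, pawn sensing and a peace, chase, attack and dead state machine.
; Damage reduces HP until death, and seeing a pawn while at peace stores it and switches to chase.
; SetState ignores changes once dead, writes the state to the AI controller's Blackboard enum and sets walk speed per state, halting movement for attack and death.
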(event OnSeePawn(PawnSensing)
  (params (Pawn :type Pawn%20Object%20Reference))
  ;[1 1 1] On See Pawn
  (if (Utilities|Enum|Equal(Enum) (Variables|Default|GetCurrentStatePawn) "NewEnumerator0")
    (Variables|Actor|SetInstigator Pawn)
    (CallFunction|SetState "NewEnumerator1")))

(event Game|Damage|EventAnyDamage
  (params (Damage :type Float%20%28single-precision%29) (DamageType :type Damage%20Type%20Object%20Reference) (InstigatedBy :type Controller%20Object%20Reference) (DamageCauser :type Actor%20Object%20Reference))
  ;[1 1 1] Enemy Damage System
  (bind _output_get (Variables|Default|SetCurrentHP (- (Variables|Default|GetCurrentHP) Damage)))
  (if (> _output_get 0.0)
    (Development|PrintString (Utilities|String|ToString(Float) (Variables|Default|GetCurrentHP)))
    (else
      (CallFunction|SetState "NewEnumerator3")
      (Development|PrintString "Enemy is Dead"))))

(event EventBeginPlay
  ;[1 1 1] Set Current HP
  (Variables|Default|SetCurrentHP (Variables|Default|GetMaxHP))
  (CallFunction|SetState "NewEnumerator0"))

(fn ConstructionScript)

(fn SetState
  (params (NewState :type BPE_EnemyState%20Enum :default "NewEnumerator0"))
  (if (Utilities|Enum|NotEqual(Enum) (Variables|Default|GetCurrentStatePawn) "NewEnumerator3")
    (bind _output_get (Variables|Default|SetCurrentStatePawn NewState))
    (Utilities|FlowControl|Sequence
      (:then_0
        (AI|Components|Blackboard|SetValueasEnum (AI|GetBlackboard (Pawn|GetController)) (Variables|Default|GetStateKey) _output_get))
      (:then_1
        (switch Utilities|FlowControl|Switch|SwitchonBPE_EnemyState (Variables|Default|GetCurrentStatePawn)
          (:NewEnumerator0
            (Variables|/Script/Engine.CharacterMovementComponent|SetMaxWalkSpeed (Variables|Character|GetCharacterMovement) 3e+02))
          (:NewEnumerator1
            (Variables|/Script/Engine.CharacterMovementComponent|SetMaxWalkSpeed (Variables|Character|GetCharacterMovement) 6e+02))
          (:NewEnumerator2
            (Variables|/Script/Engine.CharacterMovementComponent|SetMaxWalkSpeed (Variables|Character|GetCharacterMovement) 0.0 :!label _label))
          (:NewEnumerator3
            (goto _label)))))))