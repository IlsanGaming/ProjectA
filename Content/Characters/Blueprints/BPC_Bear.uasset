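; Bear character Blueprint that gives the bear a damaging attack.
; The attack collision starts disabled at BeginPlay, and the attack begin and end events switch it on and off.
; Any actor that begins overlapping it receives fixed point damage along the bear's forward direction, credited to the bear's controller, with no filtering or repeat-hit check.
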(event OnComponentBeginOverlap(AttackCollision)
  (params (OverlappedComponent :type Primitive%20Component%20Object%20Reference) (OtherActor :type Actor%20Object%20Reference) (OtherComp :type Primitive%20Component%20Object%20Reference) (OtherBodyIndex :type Integer) (bFromSweep :type Boolean) (SweepResult :type Hit%20Result%20Structure%20%28by%20ref%29))
  ;[1 1 1] Bear Attack Damage
  (Game|Damage|ApplyPointDamage OtherActor 2e+01 (Transformation|GetActorForwardVector) SweepResult (Pawn|GetController) self))

(event Custom|OnAttackBegin
  ;[1 1 1] Attack Collision On/Off
  (Collision|SetCollisionEnabled (Variables|Default|GetAttackCollision) "QueryAndPhysics"))

(event Custom|OnAttackEnd
  ;[1 1 1] Attack Collision On/Off
  (Collision|SetCollisionEnabled (Variables|Default|GetAttackCollision) "NoCollision"))

(event EventBeginPlay
  ;[1 1 1] Attack Collision On/Off
  (Collision|SetCollisionEnabled (Variables|Default|GetAttackCollision) "NoCollision"))

(fn ConstructionScript
  (|CallParentFunction))