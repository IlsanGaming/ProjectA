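; RPG game instance that stores custom variables, both global and private per player UniqueID.
; Server-gated events add, set or remove values, then call the GameMode to propagate changes and fire dispatchers on add and set.
; Server-prefixed events apply received changes.
; Private adds and sets can also be shared with the player's party, with a Shared flag preventing re-sharing, and bulk setters and getters serve the save system.
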(event EventAddCustomVariable
  (params (Variable :type Name :default "None") (Value :type Integer) (UniqueID :type Name :default "None"))
  ;[1 1 1] For Server
  (if (Networking|IsServer)
    (if (Utilities|Name|NotEqual(Name) UniqueID "None")
      (CallFunction|AddCustomVariablePrivateFunction Variable Value UniqueID false)
      (else
        (CallFunction|AddCustomVariableFunction Variable Value)))))

(event EventSetAllCustomVariablefromServer
  (params (Variables :type Array%20of%20Names) (Values :type Array%20of%20Integers))
  ;[1 1 1] Save System | Client
  (Utilities|Map|Clear (Variables|CustomVariable|GetCustomVariable))
  (for (_array_element _array_index) Variables
    (Utilities|Map|Add (Variables|CustomVariable|GetCustomVariable) _array_element (Utilities|Array|Get(acopy) Values _array_index))))

(event EventSetAllCustomVariablePrivatebyUniqueID
  (params (UniqueID :type Name :default "None") (CustomVariablePrivate :type S%20Custom%20Variable%20Array%202D%20Structure))
  ;[1 1 1] Save System | Client
  (Utilities|Map|Add (Variables|CustomVariable|GetCustomVariablePrivate) UniqueID CustomVariablePrivate))

(event EventSetAllCustomVariable
  (params (Variables :type Map%20of%20Names%20to%20Integers))
  ;[1 1 1] Save System | Server-side
  (Variables|CustomVariable|SetCustomVariable Variables))

(event EventSetAllCustomVariablePrivate
  (params (VariablesPrivate :type Map%20of%20Names%20to%20Structs))
  ;[1 1 1] Save System | Server-side
  (Variables|CustomVariable|SetCustomVariablePrivate VariablesPrivate))

(event EventServerAddCV
  (params (Variable :type Name :default "None") (Value :type Integer) (UniqueID :type Name :default "None"))
  ;[1 1 1] Receive changes from server
  (if (Utilities|Name|NotEqual(Name) UniqueID "None")
    (CallFunction|AddCustomVariablePrivateFunction Variable Value UniqueID true)
    (else
      (CallFunction|AddCustomVariableFunction Variable Value))))

(event EventSetCustomVariableValue
  (params (Variable :type Name :default "None") (Value :type Integer) (Add :type Boolean) (UniqueID :type Name :default "None"))
  ;[1 1 1] For Server
  (if (Networking|IsServer)
    (if (Utilities|Name|NotEqual(Name) UniqueID "None")
      (CallFunction|SetCustomVariableValuePrivateFunction Variable Value Add UniqueID false)
      (else
        (CallFunction|SetCustomVariableValueFunction Variable Value Add)))))

(event EventRemoveCustomVariable
  (params (Variable :type Name :default "None") (UniqueID :type Name :default "None"))
  ;[1 1 1] For Server
  (if (Networking|IsServer)
    (if (Utilities|Name|NotEqual(Name) UniqueID "None")
      (CallFunction|RemoveCustomVariablePrivateFunction Variable UniqueID)
      (else
        (CallFunction|RemoveCustomVariableFunction Variable)))))

(event EventServerSetCVValue
  (params (Variable :type Name :default "None") (Value :type Integer) (Add :type Boolean) (UniqueID :type Name :default "None"))
  ;[1 1 1] Receive changes from server
  (if (Utilities|Name|NotEqual(Name) UniqueID "None")
    (CallFunction|SetCustomVariableValuePrivateFunction Variable Value Add UniqueID true)
    (else
      (CallFunction|SetCustomVariableValueFunction Variable Value Add))))

(event EventServerRemoveCV
  (params (Variable :type Name :default "None") (UniqueID :type Name :default "None"))
  ;[1 1 1] Receive changes from server
  (if (Utilities|Name|NotEqual(Name) UniqueID "None")
    (CallFunction|RemoveCustomVariablePrivateFunction Variable UniqueID)
    (else
      (CallFunction|RemoveCustomVariableFunction Variable))))

(fn AddCustomVariableFunction
  (params (Variable :type Name) (Value :type Integer))
  (Utilities|Map|Add (Variables|CustomVariable|GetCustomVariable) Variable Value)
  (if (Networking|IsServer)
    (Utilities|FlowControl|Sequence
      (:then_0
        (Class|BPICustomVariable|ServerAddCV(Message) (Game|GetGameMode) Variable Value "None"))
      (:then_1
        (Class|BPIGameModeRPG|CallCustomDispatcherVariable(Message) (Game|GetGameMode) Variable Value false "None")))))

(fn SetCustomVariableValueFunction
  (params (Variable :type Name) (Value :type Integer) (Add :type Boolean))
  (bind _customvariable (Variables|CustomVariable|GetCustomVariable))
  (bind (_value _returnvalue) (Utilities|Map|Find _customvariable Variable))
  (if _returnvalue
    (LocalVariables|SetVarNewValue (select Add (+ Value _value) Value))
    (Utilities|Map|Add (Variables|CustomVariable|GetCustomVariable) Variable (LocalVariables|GetVarNewValue))
    (if (Networking|IsServer)
      (Utilities|FlowControl|Sequence
        (:then_0
          (Class|BPICustomVariable|ServerSetCVValue(Message) (Game|GetGameMode) Variable (LocalVariables|GetVarNewValue) false "None"))
        (:then_1
          (Class|BPIGameModeRPG|CallCustomDispatcherVariable(Message) (Game|GetGameMode) Variable (LocalVariables|GetVarNewValue) false "None"))))))

(fn AddCustomVariablePrivateFunction
  (params (Variable :type Name) (Value :type Integer) (UniqueID :type Name) (Shared :type Boolean))
  (bind _output_get (LocalVariables|SetVarValue (.Value (Utilities|Map|Find (Variables|CustomVariable|GetCustomVariablePrivate) UniqueID))))
  (if (not (Utilities|Array|ContainsItem (.Variables (Utilities|Struct|BreakS_CustomVariable_Array2D _output_get)) Variable))
    (Utilities|Array|Add (.Variables (Utilities|Struct|BreakS_CustomVariable_Array2D _output_get)) Variable)
    (Utilities|Array|Add (.Values (Utilities|Struct|BreakS_CustomVariable_Array2D _output_get)) Value)
    (Utilities|Map|Add (Variables|CustomVariable|GetCustomVariablePrivate) UniqueID (LocalVariables|GetVarValue))
    (if (Networking|IsServer)
      (Utilities|FlowControl|Sequence
        (:then_0
          (Class|BPICustomVariable|ServerAddCV(Message) (Game|GetGameMode) Variable Value UniqueID)
          (bind (_success _player) (Class|BPIGameModeRPG|GetConnectedPlayerbyUniqueID(Message) (Game|GetGameMode) UniqueID))
          (if _success
            (Utilities|IsValid _player
              (:Is%20Valid
                (if (and (not Shared) (Utilities|Array|ContainsItem (Variables|/Game/RPGSystem/Blueprints/BPC_RPGSystem.BPC_RPGSystem_C|GetVariablesToShare _player) Variable))
                  (Class|BPIGameModeRPG|ServerSharePrivateVariable(Message) (Game|GetGameMode) (Utilities|Array|MakeArray Variable) Value true UniqueID (Variables|/Game/RPGSystem/Blueprints/BPC_RPGSystem.BPC_RPGSystem_C|GetPartyID _player)))))))
        (:then_1
          (Class|BPIGameModeRPG|CallCustomDispatcherVariable(Message) (Game|GetGameMode) Variable Value true UniqueID))))))

(fn SetCustomVariableValuePrivateFunction
  (params (Variable :type Name) (Value :type Integer) (Add :type Boolean) (UniqueID :type Name%20%28by%20ref%29) (Shared :type Boolean))
  (if (Utilities|Name|NotEqual(Name) UniqueID "None")
    (bind _output_get (LocalVariables|SetVarValue (.Value (Utilities|Map|Find (Variables|CustomVariable|GetCustomVariablePrivate) UniqueID))))
    (bind _output_get_2 (LocalVariables|SetVarIndex (Utilities|Array|FindItem (.Variables (Utilities|Struct|BreakS_CustomVariable_Array2D _output_get)) Variable)))
    (if (!= _output_get_2 -1)
      (LocalVariables|SetVarNewValue (select Add (+ Value (Utilities|Array|Get(acopy) (.Values (Utilities|Struct|BreakS_CustomVariable_Array2D _output_get)) (LocalVariables|GetVarIndex))) Value))
      (|SetBy-RefVar (Utilities|Array|Get(acopy) (.Values (Utilities|Struct|BreakS_CustomVariable_Array2D _output_get)) (LocalVariables|GetVarIndex)) (LocalVariables|GetVarNewValue))
      (Utilities|Map|Add (Variables|CustomVariable|GetCustomVariablePrivate) UniqueID (LocalVariables|GetVarValue))
      (if (Networking|IsServer)
        (Utilities|FlowControl|Sequence
          (:then_0
            (Class|BPICustomVariable|ServerSetCVValue(Message) (Game|GetGameMode) Variable Value Add UniqueID)
            (bind (_success _player) (Class|BPIGameModeRPG|GetConnectedPlayerbyUniqueID(Message) (Game|GetGameMode) UniqueID))
            (if _success
              (Utilities|IsValid _player
                (:Is%20Valid
                  (if (and (not Shared) (Utilities|Array|ContainsItem (Variables|/Game/RPGSystem/Blueprints/BPC_RPGSystem.BPC_RPGSystem_C|GetVariablesToShare _player) Variable))
                    (Class|BPIGameModeRPG|ServerSharePrivateVariable(Message) (Game|GetGameMode) (Utilities|Array|MakeArray Variable) Value Add UniqueID (Variables|/Game/RPGSystem/Blueprints/BPC_RPGSystem.BPC_RPGSystem_C|GetPartyID _player)))))))
          (:then_1
            (Class|BPIGameModeRPG|CallCustomDispatcherVariable(Message) (Game|GetGameMode) Variable (LocalVariables|GetVarNewValue) true UniqueID)))))))

(fn RemoveCustomVariableFunction
  (params (Variable :type Name))
  (Utilities|Map|Remove (Variables|CustomVariable|GetCustomVariable) Variable)
  (if (Networking|IsServer)
    (if (Networking|IsDedicatedServer)
      (Class|BPICustomVariable|ServerRemoveCV(Message) (Game|GetGameMode) Variable "None")
      (else
        (Class|BPICustomVariable|ServerRemoveCV(Message) (Game|GetGameMode) Variable "None")
        (bind _reference (Class|BPIRPGSystem|GetRPGSystem(Message) (Game|GetPlayerCharacter 0)))
        (Default|UpdateQuestTask _reference Variable -1 false)))))

(fn RemoveCustomVariablePrivateFunction
  (params (Variable :type Name) (UniqueID :type Name))
  (bind _customvariableprivate (Variables|CustomVariable|GetCustomVariablePrivate))
  (bind (_value _returnvalue) (Utilities|Map|Find _customvariableprivate UniqueID))
  (if _returnvalue
    (bind _output_get (LocalVariables|SetVarValue _value))
    (bind _output_get_2 (LocalVariables|SetVarIndex (Utilities|Array|FindItem (.Variables (Utilities|Struct|BreakS_CustomVariable_Array2D _output_get)) Variable)))
    (if (!= _output_get_2 -1)
      (Utilities|Array|RemoveIndex (.variables (LocalVariables|GetVarValue)) (LocalVariables|GetVarIndex))
      (Utilities|Array|RemoveIndex (.values (LocalVariables|GetVarValue)) (LocalVariables|GetVarIndex))
      (Utilities|Map|Add (Variables|CustomVariable|GetCustomVariablePrivate) Variable (LocalVariables|GetVarValue))
      (if (Networking|IsServer)
        (Class|BPICustomVariable|ServerRemoveCV(Message) (Game|GetGameMode) Variable UniqueID)))))

(fn GetAllCustomVariable
  (return (Utilities|Struct|MakeS_All_CustomVariable (Variables|CustomVariable|GetCustomVariable) (Variables|CustomVariable|GetCustomVariablePrivate))))

(fn GetAllCustomVariablePrivatebyUniqueID
  (params (UniqueID :type Name :default "None"))
  (return (.Value (Utilities|Map|Find (Variables|CustomVariable|GetCustomVariablePrivate) UniqueID))))

(fn GetCustomVariableValue
  (params (Variable :type Name :default "None") (UniqueID :type Name :default "None"))
  (bind _customvariableprivate (Variables|CustomVariable|GetCustomVariablePrivate))
  (bind _customvariable (Variables|CustomVariable|GetCustomVariable))
  (bind (_value _returnvalue) (Utilities|Map|Find _customvariable Variable))
  (bind (_value_2 _returnvalue_2) (Utilities|Map|Find _customvariableprivate UniqueID))
  (bind (_variables _values) (Utilities|Struct|BreakS_CustomVariable_Array2D _value_2))
  (if (Utilities|Name|Equal(Name) UniqueID "None")
    (if _returnvalue
      (return true _value)
      (else
        (return false 0)))
    (elif _returnvalue_2
      (bind _output_get (LocalVariables|SetVarIndex (Utilities|Array|FindItem _variables Variable)))
      (if (!= _output_get -1)
        (return true (Utilities|Array|Get(acopy) _values (LocalVariables|GetVarIndex)))
        (else
          (return false 0)))
      (else
        (return false 0)))))