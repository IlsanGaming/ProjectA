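; Example save game object for the RPG system that holds player data, sell history, custom variables and global quest state.
; Player info is kept in separate local and server maps keyed by unique player ID, chosen by a save method.
; Paired save and load functions wrap each store, with private variables accessible whole or per unique ID.
; The functions only update or read its variables, with no disk writes here.
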(fn Save
  (params (SaveMethod :type E_SaveMethod%20Enum :default "NewEnumerator0") (UniquePlayerID :type Name%20%28by%20ref%29) (PlayerInfoSaveData :type S%20Player%20Info%20Save%20Data%20Structure))
  (switch Utilities|FlowControl|Switch|SwitchonE_SaveMethod SaveMethod
    (:NewEnumerator0
      (Utilities|Map|Add (Variables|Default|GetPlayerInfoSaveDataLocally) UniquePlayerID PlayerInfoSaveData))
    (:NewEnumerator1
      (Utilities|Map|Add (Variables|Default|GetPlayerInfoSaveDataServer) UniquePlayerID PlayerInfoSaveData))))

(fn Load
  (params (SaveMethod :type E_SaveMethod%20Enum :default "NewEnumerator0") (UniquePlayerID :type Name%20%28by%20ref%29))
  (bind _playerinfosavedatalocally (Variables|Default|GetPlayerInfoSaveDataLocally))
  (bind _playerinfosavedataserver (Variables|Default|GetPlayerInfoSaveDataServer))
  (bind (_value _returnvalue) (Utilities|Map|Find _playerinfosavedataserver UniquePlayerID))
  (bind (_value_2 _returnvalue_2) (Utilities|Map|Find _playerinfosavedatalocally UniquePlayerID))
  (switch Utilities|FlowControl|Switch|SwitchonE_SaveMethod SaveMethod
    (:NewEnumerator0
      (return _returnvalue_2 _value_2))
    (:NewEnumerator1
      (return _returnvalue _value))))

(fn SaveSellHistory
  (params (UniquePlayerID :type Name%20%28by%20ref%29) (SellHistory :type S%20Player%20Sell%20History%20Structure%20%28by%20ref%29))
  (Utilities|Map|Add (Variables|Default|GetPlayerSellHistory) UniquePlayerID SellHistory))

(fn LoadSellHistory
  (params (UniquePlayerID :type Name%20%28by%20ref%29))
  (bind _playersellhistory (Variables|Default|GetPlayerSellHistory))
  (bind (_value _returnvalue) (Utilities|Map|Find _playersellhistory UniquePlayerID))
  (return _returnvalue _value))

(fn SaveVariablePrivateUnique
  (params (UniqueID :type Name) (CustomVariablePrivate :type S%20Custom%20Variable%20Array%202D%20Structure))
  (Utilities|Map|Add (Variables|Server|GetCustomVariablePrivate) UniqueID CustomVariablePrivate))

(fn LoadVariablePrivate
  (return (Variables|Server|GetCustomVariablePrivate)))

(fn SaveVariable
  (params (CustomVariable :type Map%20of%20Names%20to%20Integers))
  (Variables|Server|SetCustomVariable CustomVariable))

(fn LoadVariable
  (return (Variables|Server|GetCustomVariable)))

(fn SaveVariablePrivate
  (params (CustomVariablePrivate :type Map%20of%20Names%20to%20Structs))
  (Variables|Server|SetCustomVariablePrivate CustomVariablePrivate))

(fn LoadVariablePrivateUnique
  (params (UniqueID :type Name))
  (return (.Value (Utilities|Map|Find (Variables|Server|GetCustomVariablePrivate) UniqueID))))

(fn SaveGlobalQuests
  (params (GlobalQuests :type Array%20of%20Names) (GlobalQuestsComplete :type Array%20of%20Names))
  (Variables|Server|SetGlobalQuests GlobalQuests)
  (Variables|Server|SetGlobalQuestsComplete GlobalQuestsComplete))

(fn LoadGlobalQuests
  (return (Variables|Server|GetGlobalQuests) (Variables|Server|GetGlobalQuestsComplete)))