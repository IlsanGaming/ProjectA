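; Base AI spawner actor that spawns data-table monsters at random navigable points inside a sphere or box area.
; An authority-side trigger overlap or game mode custom dispatcher starts a one-shot, delay-paced loop through the ToSpawn list, retrying failed spawns.
; Death callbacks feed a capped, timer-driven respawn queue and can call a finish dispatcher when spawning is exhausted.
; The construction script builds both collision volumes with configurable shapes and offsets.
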(event Custom|SnapToGround
  (bind _returnvalue (Transformation|GetActorLocation))
  (bind (_outhit _returnvalue_2) (Collision|LineTraceByChannel _returnvalue (+ _returnvalue (* (Transformation|GetActorUpVector) -1e+04)) "TraceTypeQuery1" false 0 "None"))
  (if _returnvalue_2
    (Transformation|SetActorLocation (.Location (Collision|BreakHitResult _outhit)) false true)))

(event Custom|StartLoopBody
  (bind _tospawn (Variables|Configuration|GetToSpawn))
  (bind _loopindex (Variables|Default|GetLoopIndex))
  (bind _output (Utilities|Array|Get(acopy) _tospawn _loopindex))
  ;[1 1 1] Loop Body
  (if (Utilities|Array|IsValidIndex _tospawn _loopindex)
    (Variables|Default|SetLoopData _output)
    (Utilities|Struct|SetmembersinS_Spawner_Enemy_Entry (Variables|Default|GetLoopData) 0 (Utilities|Struct|BreakS_Spawner_Enemy_Entry _output))
    (CallFunction|SpawnLoopBody)))

(event Custom|SpawnLoopBody
  (bind _loopdata (Variables|Default|GetLoopData))
  (bind _loopdata_2 (Variables|Default|GetLoopData))
  (bind (_amount _maxrespawn) (Utilities|Struct|BreakS_Spawner_Enemy_Entry _loopdata))
  ;[1 1 1] Loop Body
  (if (< _amount _maxrespawn)
    (bind _failed (CallFunction|SpawnEnemy (Variables|Default|GetLoopIndex) false))
    (if _failed
      (Utilities|FlowControl|Delay 0.02)
      (CallFunction|SpawnLoopBody)
      (else
        (Utilities|Struct|SetmembersinS_Spawner_Enemy_Entry _loopdata_2 (+ (Utilities|Struct|BreakS_Spawner_Enemy_Entry _loopdata_2) 1))
        (Utilities|FlowControl|Delay (Math|Float|Max(Float) (Variables|Configuration|GetLoopDelay) 0.0001))
        (CallFunction|SpawnLoopBody)))
    (elif (< (Variables|Default|GetLoopIndex) (- (Utilities|Array|Length (Variables|Configuration|GetToSpawn)) 1))
      (Math|Integer|IncrementInt (Variables|Default|GetLoopIndex)
        (:%20%20
          (Utilities|FlowControl|Delay (Math|Float|Max(Float) (Variables|Configuration|GetLoopDelay) 0.0001))
          (CallFunction|StartLoopBody)))
      (else
        (Variables|Default|SetLoopIndex 0)))))

(event Custom|OnKilled
  (params (Attacker :type BPC%20RPG%20System%20Object%20Reference) (Impulse :type S%20Impulse%20Structure) (Victim :type BPC%20RPG%20System%20Object%20Reference))
  ;[1 1 1] On Enemy Killed | Add to respawn list
  (bind (_succes _monsterid) (Class|BPIRPGSystem|GetEnemyInfo(Message) (Components|GetOwner Victim)))
  (if _succes
    (bind (_success _index) (CallFunction|GetMonsterIndex _monsterid))
    (if _success
      (CallFunction|SetSpawnedAmount _index -1 true)
      (bind _canrespawn (CallFunction|CanSpawn _index true))
      (if _canrespawn
        (Utilities|FlowControl|Sequence
          (:then_0
            (if (Utilities|Array|IsValidIndex (Variables|Default|GetRespawnCounter) _index)
              (|SetBy-RefVar (Utilities|Array|Get(acopy) (Variables|Default|GetRespawnCounter) _index) (+ (Utilities|Array|Get(acopy) (Variables|Default|GetRespawnCounter) _index) 1))
              (else
                (Utilities|Array|SetArrayElem (Variables|Default|GetRespawnCounter) _index 1 true))))
          (:then_1
            (Utilities|Array|Add (Variables|Default|GetRespawnQueue) (Utilities|Struct|MakeS_Spawner_RespawnQueue_Entry _index (Utilities|Time|GetGameTimeinSeconds)))
            (if (not (Utilities|Time|IsTimerActivebyHandle (Variables|Default|GetTimer)))
              (bind _returnvalue (Utilities|Time|SetTimerbyFunctionName self "RespawnEnemy" (Variables|Configuration|GetRespawnTime)))
              (Variables|Default|SetTimer _returnvalue))))
        (elif (and (<= (Utilities|Array|Length (Variables|Default|GetRespawnQueue)) 0) (<= (CallFunction|GetSpawnedAmount) 0))
          (if (Utilities|Name|NotEqual(Name) (Variables|Configuration|GetCustomDispatcherCallOnFinish) "None")
            (Class|BPIGameModeRPG|CallCustomDispatcher(Message) (Game|GetGameMode) (Variables|Configuration|GetCustomDispatcherCallOnFinish) "None" "None")))))))

(event Custom|OnBeginOverlap
  (params (OverlappedComponent :type Primitive%20Component%20Object%20Reference) (OtherActor :type Actor%20Object%20Reference) (OtherComp :type Primitive%20Component%20Object%20Reference) (OtherBodyIndex :type Integer) (bFromSweep :type Boolean) (SweepResult :type Hit%20Result%20Structure%20%28by%20ref%29))
  ;[1 1 1] OnTrigger
  (Networking|SwitchHasAuthority
    (:Authority
      (if (not (Variables|Default|GetTriggered))
        (bind _success (Class|BPIRPGSystem|GetRPGSystem(Message) OtherActor))
        (if _success
          (Variables|Default|SetTriggered true)
          (CallFunction|StartLoopBody))))))

(event EventOnCustomDispatcherPrivate
  (params (DispatcherID :type Name :default "None") (Message :type Name :default "None") (UniqueID :type Name :default "None"))
  (if (not (Variables|Default|GetTriggered))
    (Variables|Default|SetTriggered true)
    (CallFunction|StartLoopBody)))

(event EventBeginPlay
  (bind _triggercustomdispatcher (Variables|Configuration|GetTriggerCustomDispatcher))
  ;[1 1 1] Trigger Dispatcher
  (Networking|SwitchHasAuthority
    (:Authority
      (if (Utilities|Name|NotEqual(Name) _triggercustomdispatcher "None")
        (Class|BPIGameModeRPG|BindCustomDispatcher(Message) (Game|GetGameMode) self _triggercustomdispatcher)))))

(event EventOnCustomDispatcher
  (params (DispatcherID :type Name :default "None") (Message :type Name :default "None"))
  (if (not (Variables|Default|GetTriggered))
    (Variables|Default|SetTriggered true)
    (CallFunction|StartLoopBody)))

(fn ConstructionScript
  (CallFunction|UpdateSpawnerCollisionType)
  (CallFunction|UpdateTriggerCollisionType)
  (CallFunction|TriggerOffsetUpdate))

(fn OnRepCollisionType
  (CallFunction|UpdateSpawnerCollisionType))

(fn UpdateSpawnerCollisionType
  (switch Utilities|FlowControl|Switch|SwitchonE_SkillTraceType (Variables|Configuration|GetSpawnerCollisionType)
    (:NewEnumerator0
      (Utilities|IsValid (Variables|Components|GetSpawnerBoxCollision)
        (:Is%20Valid
          (Components|DestroyComponent (Variables|Components|GetSpawnerBoxCollision)))
        (:Is%20Not%20Valid
          _))
      (bind _returnvalue (AddComponent|AddSphereComponent false))
      (Components|Sphere|SetSphereRadius _returnvalue (Variables|Configuration|GetSpawnerSphereRange) false)
      (Variables|Components|SetSpawnerSphereCollision _returnvalue))
    (:NewEnumerator1
      (Utilities|IsValid (Variables|Components|GetSpawnerSphereCollision)
        (:Is%20Valid
          (Components|DestroyComponent (Variables|Components|GetSpawnerSphereCollision)))
        (:Is%20Not%20Valid
          _))
      (bind _returnvalue_2 (AddComponent|AddBoxComponent false))
      (Components|Box|SetBoxExtent _returnvalue_2 (Variables|Configuration|GetSpawnerBoxRange) false)
      (Variables|Components|SetSpawnerBoxCollision _returnvalue_2))))

(fn OnRepSphereRange
  (if (Utilities|Enum|Equal(Enum) (Variables|Configuration|GetSpawnerCollisionType) "NewEnumerator0")
    (Utilities|IsValid (Variables|Components|GetSpawnerSphereCollision)
      (:Is%20Valid
        (Components|Sphere|SetSphereRadius (Variables|Components|GetSpawnerSphereCollision) (Variables|Configuration|GetSpawnerSphereRange) false)))))

(fn OnRepBoxRange
  (if (Utilities|Enum|Equal(Enum) (Variables|Configuration|GetSpawnerCollisionType) "NewEnumerator1")
    (Utilities|IsValid (Variables|Components|GetSpawnerBoxCollision)
      (:Is%20Valid
        (Components|Box|SetBoxExtent (Variables|Components|GetSpawnerBoxCollision) (Variables|Configuration|GetSpawnerBoxRange) false)))))

(fn UpdateTriggerCollisionType
  (if (Variables|Configuration|GetDisableTriggerCollision)
    (Utilities|FlowControl|Sequence
      (:then_0
        (Utilities|IsValid (Variables|Components|GetTriggerBoxCollision)
          (:Is%20Valid
            (Components|DestroyComponent (Variables|Components|GetTriggerBoxCollision)))))
      (:then_1
        (Utilities|IsValid (Variables|Components|GetTriggerSphereCollision)
          (:Is%20Valid
            (Components|DestroyComponent (Variables|Components|GetTriggerSphereCollision))))))
    (else
      (switch Utilities|FlowControl|Switch|SwitchonE_SkillTraceType (Variables|Configuration|GetTriggerCollisionType)
        (:NewEnumerator0
          (Utilities|IsValid (Variables|Components|GetTriggerBoxCollision)
            (:Is%20Valid
              (Components|DestroyComponent (Variables|Components|GetTriggerBoxCollision)))
            (:Is%20Not%20Valid
              _))
          (bind _returnvalue (AddComponent|AddSphereComponent false))
          (Components|Sphere|SetSphereRadius _returnvalue (Variables|Configuration|GetTriggerSphereRange) false)
          (bind _output_get (Variables|Components|SetTriggerSphereCollision _returnvalue))
          (Collision|BindEventtoOnComponentBeginOverlap _output_get (EventDispatchers|CreateEvent :!event Custom|OnBeginOverlap)))
        (:NewEnumerator1
          (Utilities|IsValid (Variables|Components|GetTriggerSphereCollision)
            (:Is%20Valid
              (Components|DestroyComponent (Variables|Components|GetTriggerSphereCollision)))
            (:Is%20Not%20Valid
              _))
          (bind _returnvalue_2 (AddComponent|AddBoxComponent false))
          (Components|Box|SetBoxExtent _returnvalue_2 (Variables|Configuration|GetTriggerBoxRange) false)
          (bind _output_get_2 (Variables|Components|SetTriggerBoxCollision _returnvalue_2))
          (Collision|BindEventtoOnComponentBeginOverlap _output_get_2 (EventDispatchers|CreateEvent :!event Custom|OnBeginOverlap)))))))

(fn RespawnEnemy
  (bind _respawnqueue (Variables|Default|GetRespawnQueue))
  (bind _failed (CallFunction|SpawnEnemy (.MonsterIndex (Utilities|Struct|BreakS_Spawner_RespawnQueue_Entry (Utilities|Array|Get(acopy) (Variables|Default|GetRespawnQueue)))) false))
  (if _failed
    (Utilities|Time|SetTimerbyFunctionName self "RespawnEnemy" 0.2)
    (else
      (Utilities|Array|RemoveIndex _respawnqueue)
      (if (> (Utilities|Array|Length _respawnqueue) 0)
        (bind _returnvalue (Utilities|Time|SetTimerbyFunctionName self "RespawnEnemy" (Math|Float|Max(Float) (- (Variables|Configuration|GetRespawnTime) (- (Utilities|Time|GetGameTimeinSeconds) (.KillTime (Utilities|Struct|BreakS_Spawner_RespawnQueue_Entry (Utilities|Array|Get(acopy) (Variables|Default|GetRespawnQueue)))))) 0.5)))
        (Variables|Default|SetTimer _returnvalue)))))

(fn SpawnEnemy
  (params (Index :type Integer) (Startup :type Boolean))
  (Utilities|FlowControl|Sequence
    (:then_0
      (switch Utilities|FlowControl|Switch|SwitchonE_SkillTraceType (Variables|Configuration|GetSpawnerCollisionType)
        (:NewEnumerator0
          (LocalVariables|SetVarOrigin (Transformation|GetWorldLocation (Variables|Components|GetSpawnerSphereCollision)))
          (LocalVariables|SetVarRadius (* (Variables|Configuration|GetSpawnerSphereRange) 2.0)))
        (:NewEnumerator1
          (LocalVariables|SetVarOrigin (Math|Random|RandomPointinBoundingBox (Transformation|GetWorldLocation (Variables|Components|GetSpawnerBoxCollision)) (Variables|Configuration|GetSpawnerBoxRange)))
          (LocalVariables|SetVarRadius 1e+01))))
    (:then_1
      (bind (_randomlocation _returnvalue) (Class|NavigationSystemV1|GetRandomLocationinNavigableRadius (LocalVariables|GetVarOrigin) (LocalVariables|GetVarRadius) 0 0))
      (Variables|Default|SetNewVar_0 _randomlocation)
      (if _returnvalue
        (bind (_success _returnvalue_2) (CallFunction|SpawnMonsterfromDatatable (Utilities|Struct|BreakS_Spawner_Enemy_Entry (Utilities|Array|Get(acopy) (Variables|Configuration|GetToSpawn) Index)) (+ (Variables|Default|GetNewVar_0) "0, 0,250.000000") (Math|Rotator|MakeRotator 0.0 0.0 (Math|Random|RandomFloatinRange -1.8e+02 1.8e+02)) true))
        (if _success
          (bind _reference (Class|BPIRPGSystem|GetRPGSystemAI(Message) _returnvalue_2))
          (EventDispatchers|BindEventtoOnDeath _reference (EventDispatchers|CreateEvent :!event Custom|OnKilled))
          (if Startup
            _
            (else
              (CallFunction|SetSpawnedAmount Index 1 true)))
          (return false)
          (else
            (return true)))
        (else
          (return true))))))

(fn GetMonsterIndex
  (params (MonsterID :type Name))
  (for (_array_element _array_index) (Variables|Configuration|GetToSpawn)
    (if (Utilities|Name|Equal(Name) (Utilities|Struct|BreakS_Spawner_Enemy_Entry _array_element) MonsterID)
      (return true _array_index)))
  (return false 0))

(fn CanSpawn
  (params (Index :type Integer) (ForRespawn :type Boolean))
  (bind _respawncounter (Variables|Default|GetRespawnCounter))
  (bind _tospawn (Variables|Configuration|GetToSpawn))
  (bind _spawnedcounter (Variables|Default|GetSpawnedCounter))
  (bind _output (Utilities|Array|Get(acopy) _spawnedcounter Index))
  (bind _output_2 (Utilities|Array|Get(acopy) _tospawn Index))
  (bind (_monsterid _amount _maxrespawn) (Utilities|Struct|BreakS_Spawner_Enemy_Entry _output_2))
  (bind _returnvalue (< _output _amount))
  (if ForRespawn
    (if (Utilities|Array|IsValidIndex _respawncounter Index)
      (return (< (Utilities|Array|Get(acopy) _respawncounter Index) _maxrespawn))
      (else
        (return true)))
    (elif (Utilities|Array|IsValidIndex _spawnedcounter Index)
      (if _returnvalue
        (return _returnvalue)
        (else
          (return false)))
      (else
        (return true)))))

(fn GetRespawnTime
  (params (QueueIndex :type Integer))
  (return (Math|Float|Max(Float) (- (Variables|Configuration|GetRespawnTime) (- (Utilities|Time|GetGameTimeinSeconds) (.KillTime (Utilities|Struct|BreakS_Spawner_RespawnQueue_Entry (Utilities|Array|Get(acopy) (Variables|Default|GetRespawnQueue) QueueIndex))))) 0.5)))

(fn TriggerOffsetUpdate
  (bind _triggeroffset (Variables|Configuration|GetTriggerOffset))
  (bind _spawneroffset (Variables|Configuration|GetSpawnerOffset))
  (Utilities|FlowControl|Sequence
    (:then_0
      (if (not (Variables|Configuration|GetDisableTriggerCollision))
        (switch Utilities|FlowControl|Switch|SwitchonE_SkillTraceType (Variables|Configuration|GetTriggerCollisionType)
          (:NewEnumerator0
            (Transformation|SetRelativeLocation (Variables|Components|GetTriggerSphereCollision) _triggeroffset false true))
          (:NewEnumerator1
            (Transformation|SetRelativeLocation (Variables|Components|GetTriggerBoxCollision) _triggeroffset false true)))))
    (:then_1
      (switch Utilities|FlowControl|Switch|SwitchonE_SkillTraceType (Variables|Configuration|GetSpawnerCollisionType)
        (:NewEnumerator0
          (Transformation|SetRelativeLocation (Variables|Components|GetSpawnerSphereCollision) _spawneroffset false true))
        (:NewEnumerator1
          (Transformation|SetRelativeLocation (Variables|Components|GetSpawnerBoxCollision) _spawneroffset false true))))))

(fn SetSpawnedAmount
  (params (Index :type Integer) (Amount :type Integer) (Add :type Boolean))
  (bind _spawnedcounter (Variables|Default|GetSpawnedCounter))
  (bind _output (Utilities|Array|Get(acopy) _spawnedcounter Index))
  (if (Utilities|Array|IsValidIndex (Variables|Default|GetSpawnedCounter) Index)
    (if Add
      (|SetBy-RefVar _output (+ _output Amount))
      (elif (not (<= Amount 0))
        (Utilities|Array|SetArrayElem (Variables|Default|GetSpawnedCounter) Index Amount true :!label _label)))
    (elif (not (<= Amount 0))
      (goto _label))))

(fn OnRepDisableTriggerCollision
  (CallFunction|UpdateTriggerCollisionType))

(fn GetSpawnedAmount
  (for _array_element (Variables|Default|GetSpawnedCounter)
    (LocalVariables|SetVarAmount _array_element))
  (return (LocalVariables|GetVarAmount)))