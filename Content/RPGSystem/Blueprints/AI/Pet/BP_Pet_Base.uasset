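; Base character for RPG system AI pets, whose blackboard target is expected to be an item actor.
; Server-side Tick caches the falling state and smoothly rotates the pet along its velocity, or toward the target item when stationary or, if look-lock is enabled, close.
; Unpossessing expires the old controller almost immediately.
; Shared query functions expose movement and capsule radius, while enemy, equipment and RPG-system ones are empty stubs.
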(event EventTick
  (params (DeltaSeconds :type Float%20%28single-precision%29))
  (bind _returnvalue (Transformation|GetActorRotation))
  (bind _returnvalue_2 (Transformation|GetVelocity))
  (bind _returnvalue_3 (Transformation|GetActorLocation))
  (bind _self self)
  (bind _returnvalue_4 (AI|GetAIController _self))
  (bind _returnvalue_5 (Math|Vector|VectorLength _returnvalue_2))
  (bind _returnvalue_6 (* _returnvalue_2 1e+01))
  (bind _returnvalue_7 (AI|GetBlackboard _returnvalue_4))
  (bind _returnvalue_8 (> _returnvalue_5 1e+01))
  (bind _returnvalue_9 (+ _returnvalue_3 _returnvalue_6))
  ;[1 1 1] Smooth Rotation
  (if (Networking|IsServer)
    (Variables|Default|SetFalling (AI|Components|NavMovement|IsFalling (Variables|Character|GetCharacterMovement)))
    (Utilities|IsValid (AI|GetAIController self)
      (:Is%20Valid
        (if (ScalableFloat|GetValueasBool _returnvalue_7 (Utilities|Name|MakeLiteralName "HasTarget"))
          (if (Variables|Default|GetLockLookAtTargetClose)
            (if (< (CallFunction|GetDistanceXY (Transformation|GetActorLocation) (AI|Components|Blackboard|GetValueasVector _returnvalue_7 (Utilities|Name|MakeLiteralName "TargetLocation"))) (+ (* (Components|Capsule|GetScaledCapsuleRadius (Variables|Collision|GetCapsuleComponent)) 3.0) 1e+02))
              (bind _asbp_item_base (Utilities|Casting|CastToBP_Item_Base (AI|Components|Blackboard|GetValueasObject _returnvalue_7 (Utilities|Name|MakeLiteralName "Target")) :!label _label))
              (Variables|Default|SetLookAt (Transformation|GetActorLocation _asbp_item_base))
              (else
                (if _returnvalue_8 :!label _label_2
                  (Variables|Default|SetLookAt _returnvalue_9)
                  (else
                    (goto _label)))))
            (else
              (goto _label_2)))
          (Transformation|SetActorRotation (Class|KismetMathLibrary|RInterptoConstant _returnvalue (Math|Rotator|MakeRotator (.Roll (Math|Rotator|BreakRotator (Math|Rotator|FindLookatRotation (Transformation|GetActorLocation) (Variables|Default|GetLookAt)))) (.Pitch (Math|Rotator|BreakRotator _returnvalue)) (.Yaw (Math|Rotator|BreakRotator (Math|Rotator|FindLookatRotation (Transformation|GetActorLocation) (Variables|Default|GetLookAt))))) DeltaSeconds (* 4.0 (Math|Float|MakeLiteralFloat 1e+02))) :!label _label_3)
          (elif _returnvalue_8
            (Variables|Default|SetLookAt _returnvalue_9)
            (goto _label_3)))))))

(event EventUnpossessed
  (params (OldController :type Controller%20Object%20Reference))
  (Actor|SetLifeSpan OldController 0.01))

(fn ConstructionScript)

(fn GetCapsuleHalfHeight
  (return 0.0))

(fn GetEnemyInfo
  (return false "None" "" "" ""))

(fn GetMeshRadius
  (return (Components|Capsule|GetScaledCapsuleRadius (Variables|Collision|GetCapsuleComponent))))

(fn GetMovementSpeed
  (return (Variables|/Script/Engine.CharacterMovementComponent|GetMaxWalkSpeed (Variables|Character|GetCharacterMovement))))

(fn GetPlayerSkeletalMesh
  (return false 0))

(fn GetRPGSystem
  (return false 0))

(fn GetRPGSystemAI
  (return false 0))

(fn IsDualWield
  (return false))

(fn IsFalling
  (return (Variables|Default|GetFalling)))

(fn IsTwohanded
  (return false))

(fn SetMovementSpeed
  (params (ToDefault :type Boolean) (Speed :type Float%20%28double-precision%29))
  (Variables|/Script/Engine.CharacterMovementComponent|SetMaxWalkSpeed (Variables|Character|GetCharacterMovement) (Math|Float|SelectFloat 8e+02 Speed ToDefault)))

(fn VisualEquipmentAddSkeletalMeshComponent
  (return 0))

(fn VisualEquipmentAddStaticMeshComponent
  (return 0))