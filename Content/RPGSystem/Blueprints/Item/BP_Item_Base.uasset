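; Base actor for pickup items lying in the world, with grade-colored particles, name tooltip and outline on selection.
; Persistent items build their item struct on the server at BeginPlay.
; Interact adds the item and its custom variables to the RPGSystem inventory server-side, keeping any leftover stack or destroying the actor.
; The server simulates physics while clients ease toward its transform, then tick, physics and movement replication stop after a delay.
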(event EventSelectInteractable
  (params (Selected :type Boolean))
  ;[1 1 1] Outline
  (Rendering|SetRenderCustomDepth (Variables|Default|GetStaticMesh) Selected))

(event EventBeginPlay
  ;[1 1 1] Begin Play
  (Networking|SwitchHasAuthority
    (:Authority
      (if (Variables|Configuration|GetPersistant)
        (Variables|Configuration|SetItem (.Inventory%20Struct (CallFunction|CreateItem (Variables|Configuration|GetItem) -1.0)))
        (Variables|RunTime|SetNewDrop true)))
    (:Remote
      _))
  (Utilities|FlowControl|Sequence
    (:then_0
      (CallFunction|SetItemName)
      (|SetParticleColor))
    (:then_1
      (|SetSimulation)
      (|Replication))
    (:then_2
      (Variables|RunTime|SetCreated true))))

(event EventTick
  (params (DeltaSeconds :type Float%20%28single-precision%29))
  (bind _staticmesh (Variables|Default|GetStaticMesh))
  ;[1 1 1] Comment
  (Networking|SwitchHasAuthority
    (:Authority
      (Variables|RunTime|SetTransform (Transformation|GetWorldTransform (Variables|Default|GetStaticMesh))))
    (:Remote
      (Transformation|SetWorldTransform _staticmesh (Math|Interpolation|Ease "EaseIn" 0.96 (Transformation|GetWorldTransform _staticmesh) (Variables|RunTime|GetTransform) 2e+01) true true))))

(event EventInteract
  (params (RPGSystem :type BPC%20RPG%20System%20Object%20Reference) (Command :type String))
  ;[1 1 1] Interact
  (Utilities|IsValid RPGSystem
    (:Is%20Valid
      (Networking|SwitchHasAuthority
        (:Authority
          (if (Variables|Configuration|GetPersistant)
            (if (Variables|RunTime|GetCreated)
              (bind (_global _private) (CallFunction|GetCustomVariables :!label _label))
              (bind (_success _stackleft) (Default|InventoryAddItem RPGSystem (Variables|Configuration|GetItem) _global _private))
              (if _success
                (if (> _stackleft 0)
                  (Utilities|Struct|SetmembersinS_Inventory (Variables|Configuration|GetItem) _stackleft)
                  (Default|CallOnItemCountUpdated)
                  (CallFunction|SetItemName)
                  (else
                    (Default|CallOnLooted)
                    (Actor|DestroyActor)))))
            (else
              (goto _label))))))))

(fn ConstructionScript)

(fn SetItemName
  (bind _item (Variables|Configuration|GetItem))
  (bind _item_2 (Variables|Configuration|GetItem))
  (bind (_refinelevel _count) (Utilities|Struct|BreakS_Inventory _item))
  (bind (_itemid _gradelevel) (Utilities|Struct|BreakS_Inventory _item_2))
  (bind _returnvalue (Utilities|GetDataTableRow "/Game/RPGSystem/Blueprints/Database/DT_Item.DT_Item" _itemid)
    (:then
      (Variables|RunTime|SetItemName (CallFunction|GetItemName _returnvalue (Utilities|Enum|ByteToEnumE_ItemGrade (Math|Conversions|ToByte(Integer) _gradelevel)) _refinelevel (Math|Integer|SelectInt _count 0 (.Stackable (Utilities|Struct|BreakS_Item _returnvalue)))))
      (Variables|RunTime|SetItemType (.ItemType (Utilities|Struct|BreakS_Item _returnvalue))))))

(fn GetCustomVariables
  (LocalVariables|SetVarCustomVariables (Variables|Configuration|GetCustomVariables))
  (LocalVariables|SetVarCustomVariablesPrivate (Variables|Configuration|GetCustomVariablesPrivate))
  (for _array_element (Variables|Configuration|GetCustomVariablesTags)
    (Utilities|Array|Add (LocalVariables|GetVarCustomVariables) (GameplayTags|GetTagName _array_element)))
  (for _array_element_2 (Variables|Configuration|GetCustomVariablesTagsPrivate)
    (Utilities|Array|Add (LocalVariables|GetVarCustomVariablesPrivate) (GameplayTags|GetTagName _array_element_2)))
  (return (Utilities|Struct|MakeS_ArrayOf_FName (LocalVariables|GetVarCustomVariables)) (Utilities|Struct|MakeS_ArrayOf_FName (LocalVariables|GetVarCustomVariablesPrivate))))

(fn GetInteractInfo
  (params (RPGSystem :type BPC%20RPG%20System%20Object%20Reference))
  (bind _worldlocation (CallFunction|GetMovetoEndDestination))
  (return true (select (<= (CallFunction|GetDistanceXY (Transformation|GetActorLocation (Components|GetOwner RPGSystem)) _worldlocation) (Math|Float|SelectFloat 1.6e+02 425.0 (Variables|/Game/RPGSystem/Blueprints/BPC_RPGSystem.BPC_RPGSystem_C|GetTopDown RPGSystem))) "NewEnumerator0" "NewEnumerator1")))

(fn GetItemInfo
  (bind (_global _private) (CallFunction|GetCustomVariables))
  (return true (Variables|Configuration|GetItem) (Variables|RunTime|GetItemType) _global _private))

(fn GetMovetoEndDestination
  (return true (Transformation|GetWorldLocation (Variables|Default|GetStaticMesh))))

(fn GetScreenTooltipInfo
  (params (RPGSystem :type BPC%20RPG%20System%20Object%20Reference))
  (bind _action (CallFunction|GetInteractInfo RPGSystem))
  (return true (Utilities|Select :Index _action :NewEnumerator0 "Pickup [E]" :NewEnumerator1 "Too far away" :NewEnumerator2 "") "(R=1.000000,G=1.000000,B=1.000000,A=1.000000)"))

(fn GetWorldTooltipInfo
  (return true true (Variables|RunTime|GetItemName) (CallFunction|GetGradeColor "NewEnumerator0" (Utilities|Struct|BreakS_Inventory (Variables|Configuration|GetItem)) true) "0, 0, 0"))