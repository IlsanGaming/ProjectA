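; Main actor of the Mage Meteor Shower skill, which fires a timed volley of meteor projectiles from its location.
; On SkillStart it derives attack from skill base damage plus a non-linear bonus from the owner's INT.
; A delay loop rolls slightly randomized damage, cut for AI-controlled owners, into SkillInfo for each spawned BP_Skill_MeteorShowerProjectile.
; The actor destroys itself once the bolt count runs out.
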(event EventSkillStart
  (bind _skillowner (Variables|Default|GetSkillOwner))
  (bind _playerinfo (Variables|/Game/RPGSystem/Blueprints/BPC_RPGSystem.BPC_RPGSystem_C|GetPlayerInfo _skillowner))
  (bind _stats (Utilities|Struct|BreakS_PlayerInfo _playerinfo))
  (bind _int (Utilities|Struct|BreakS_Stats _stats))
  (bind _returnvalue (Math|Conversions|ToFloat(Integer) _int))
  (Variables|Default|SetBoltAmount 25)
  (Variables|Default|SetATK (+ (Utilities|Struct|BreakS_Skill (Variables|Default|GetSkillInfo)) (* (* (|((int*5)*((int/30)+1)) _returnvalue) (+ (/ _returnvalue 1e+02) 1.0)) 0.5)))
  (Utilities|Struct|SetmembersinS_Skill (Variables|Default|GetSkillInfo) (* (Math|Random|RandomFloatinRange (* (Variables|Default|GetATK) 0.95) (Variables|Default|GetATK)) (Math|Float|SelectFloat 0.25 1.0 (Variables|/Game/RPGSystem/Blueprints/BPC_RPGSystem.BPC_RPGSystem_C|GetPlayerAI (Variables|Default|GetSkillOwner)))) :!label _label) ; Random damange in range
  (Game|SpawnActorfromClass "/Game/RPGSystem/Blueprints/Skill/Mage/MeteorShower/BP_Skill_MeteorShowerProjectile.BP_Skill_MeteorShowerProjectile_C" (Math|Transform|MakeTransform (Transformation|GetActorLocation) "0, 0, 0" "1.000000,1.000000,1.000000") "AlwaysSpawn" "OverrideRootScale" 0 (Variables|Default|GetSkillInfo) (Variables|Default|GetSkillOwner) (Variables|Default|GetSkillLevel) (Variables|Default|GetSkillID) 0 (Variables|Default|GetKey) 0)
  (Math|Integer|DecrementInt (Variables|Default|GetBoltAmount)
    (:%20%20
      (if (> (Variables|Default|GetBoltAmount) 0)
        (Utilities|FlowControl|Delay 0.35)
        (goto _label)
        (else
          (Actor|DestroyActor))))))

(fn ConstructionScript
  (|CallParentFunction))