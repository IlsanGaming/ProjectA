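; Client-side meteor projectile for the Mage's Meteor Shower skill, with no damage logic of its own.
; On BeginPlay it activates its particles and runs a timeline that lerps it from StartLocation to EndLocation.
; On arrival it spawns an impact emitter, ends trails and destroys itself after a short delay.
; Any RangeIndicator is pinned to EndLocation and removed on impact, but the decal spawn that would create it is disconnected.
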(event Custom|Start
  (bind _particlesystem (Variables|Default|GetParticleSystem))
  (bind _rangeindicator (Variables|Default|GetRangeIndicator))
  (bind _rangeindicator_2 (Variables|Default|GetRangeIndicator))
  (bind _newtrack_0 (Timeline|BoltMovement PlayFromStart)
    (:Update
      (Utilities|IsValid _rangeindicator_2
        (:Is%20Valid
          (Transformation|SetWorldLocation _rangeindicator_2 (Variables|Default|GetEndLocation) false true))
        (:Is%20Not%20Valid
          _))
      (Transformation|SetActorLocation (Math|Vector|Lerp(Vector) (Variables|Default|GetStartLocation) (Variables|Default|GetEndLocation) _newtrack_0) false true))
    (:Finished
      (Utilities|FlowControl|DoOnce false
        (:Completed
          (Effects|SpawnEmitteratLocation "/Game/RPGSystem/Particles/P_MeteorImpact.P_MeteorImpact" (Transformation|GetActorLocation))
          (Utilities|FlowControl|Sequence
            (:then_0
              (Utilities|IsValid _rangeindicator
                (:Is%20Valid
                  (Components|DestroyComponent _rangeindicator))))
            (:then_1
              (Utilities|IsValid _particlesystem
                (:Is%20Valid
                  (Effects|Particles|Trails|EndTrails _particlesystem))
                (:Is%20Not%20Valid
                  _))
              (Utilities|FlowControl|Delay 2.0)
              (Actor|DestroyActor))))))))

(event EventBeginPlay
  (Transformation|SetActorLocation (Variables|Default|GetStartLocation) false true)
  (CallFunction|Start)
  (Components|Activation|SetActive (Variables|Default|GetParticleSystem) true false))

(fn ConstructionScript
  (|CallParentFunction))