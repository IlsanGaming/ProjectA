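; BP_Skill_WirbleStorm is a Mage skill that releases a burst of BP_Skill_Wirble modules in a ring around itself.
; On SkillStart it stores the skill info, then loops to spawn each module through SkillOwner, passing that info along and calling SkillEnd within the loop.
; Yaw fans out from the actor's facing in alternating 45-degree steps, with each spawn pushed slightly forward along its own direction.
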(event EventSkillStart
  (bind (_x _y) (Math|Vector2D|BreakVector2D "(X=50.000000,Y=0.000000)"))
  (bind _returnvalue (Transformation|GetActorRotation))
  (bind _returnvalue_2 (Math|Float|MakeLiteralFloat 45.0))
  (bind _skillowner (Variables|Default|GetSkillOwner))
  (bind (_roll _pitch _yaw) (Math|Rotator|BreakRotator _returnvalue))
  ;[1 1 1] Comment
  (Utilities|Struct|SetmembersinS_Skill (Variables|Default|GetSkillInfo))
  (for _index (range 0 8)
    (Default|SpawnSkillModule (Variables|Default|GetSkillOwner) "/Game/RPGSystem/Blueprints/Skill/Mage/BP_Skill_Wirble.BP_Skill_Wirble_C" (Math|Transform|MakeTransform (+ (Transformation|GetActorLocation) (* (Math|Vector|GetForwardVector (Math|Rotator|MakeRotator _roll _pitch (+ _yaw (select (== (Math|Integer|%(Integer) (+ _index 1) 2) 0) (* (- _index (/ _index 2)) _returnvalue_2) (* (- _index (/ _index 2)) (* _returnvalue_2 -1.0)))))) _x) (* (Math|Vector|GetUpVector (Math|Rotator|MakeRotator _roll _pitch (+ _yaw (select (== (Math|Integer|%(Integer) (+ _index 1) 2) 0) (* (- _index (/ _index 2)) _returnvalue_2) (* (- _index (/ _index 2)) (* _returnvalue_2 -1.0)))))) _y)) (Math|Rotator|MakeRotator _roll _pitch (+ _yaw (select (== (Math|Integer|%(Integer) (+ _index 1) 2) 0) (* (- _index (/ _index 2)) _returnvalue_2) (* (- _index (/ _index 2)) (* _returnvalue_2 -1.0))))) "1.000000,1.000000,1.000000") "AlwaysSpawn" (Variables|Default|GetSkillInfo) _skillowner "None" 0 (Components|GetOwner _skillowner) 0 "None")
    (CallFunction|SkillEnd)))

(fn ConstructionScript
  (|CallParentFunction))