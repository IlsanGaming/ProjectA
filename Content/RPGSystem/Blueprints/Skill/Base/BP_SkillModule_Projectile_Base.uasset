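; Base projectile skill module for the RPG skill system, moving at the skill's projectile speed until it hits something or reaches maximum range.
; Tick runs box traces over the distance travelled instead of relying on overlap events.
; Optional homing eases rotation toward the target, and the server can pick a replacement by range and angle.
; On collision, the server stops movement and starts the skill or destroys single-target misses, while clients hide the actor.
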(event Custom|OnCollided
  (params (Target :type BPC%20RPG%20System%20Object%20Reference))
  ;[1 1 1] OnCollided
  (if (not (Variables|Default|GetTriggered))
    (Variables|Default|SetTriggered true)
    (Networking|SwitchHasAuthority
      (:Authority
        (bind _output_get (Variables|Default|SetTarget Target))
        (Components|Activation|SetActive (Variables|Default|GetProjectileMovement) false false)
        (Utilities|IsValid _output_get
          (:Is%20Valid
            (Utilities|Struct|SetmembersinS_Impulse (Variables|Default|GetImpulseInfo) (Transformation|GetActorLocation))
            (CallFunction|SkillStart :!label _label))
          (:Is%20Not%20Valid
            (if (.SingleTarget (Utilities|Struct|BreakS_Skill (Variables|Default|GetSkillInfo)))
              (Actor|DestroyActor)
              (else
                (goto _label))))))
      (:Remote
        (Components|Tick|SetComponentTickEnabled (Variables|Default|GetProjectileMovement) false)
        (Rendering|SetActorHiddenInGame true)))))

(event EventSkillInitialized)

(event EventTick
  (params (DeltaSeconds :type Float%20%28single-precision%29))
  (bind _returnvalue (Transformation|GetActorRotation))
  (bind _returnvalue_2 (Transformation|GetVelocity))
  (bind _returnvalue_3 (Transformation|GetActorLocation))
  (bind _tracedistance (Variables|Projectile|GetTraceDistance))
  (bind _projectilemovement (Variables|Default|GetProjectileMovement))
  (bind _target (Variables|Default|GetTarget))
  (bind _returnvalue_4 (Components|GetOwner _target))
  (bind (_roll _pitch _yaw) (Math|Rotator|BreakRotator _returnvalue))
  (bind _returnvalue_5 (Math|Vector|VectorLength _returnvalue_2))
  (bind _returnvalue_6 (Transformation|GetActorLocation _returnvalue_4))
  ;[1 1 1] Tick
  (if (>= (Utilities|GetDistanceLocation (Variables|Temp|GetStartLocation) (Transformation|GetActorLocation)) (Variables|Default|GetPlayerAttackDistanceUnits))
    (CallFunction|CollisionTrace (Variables|Temp|GetLastTraceLocation) (Utilities|GetDistanceLocation (Variables|Temp|GetLastTraceLocation) (Transformation|GetActorLocation)))
    (CallFunction|OnCollided)
    (else
      (if (>= (Utilities|GetDistanceLocation (Variables|Temp|GetLastTraceLocation) (Transformation|GetActorLocation)) (Math|Float|SelectFloat (* _returnvalue_5 0.5) _tracedistance (< _returnvalue_5 _tracedistance)))
        (CallFunction|CollisionTrace (Variables|Temp|GetLastTraceLocation) (Utilities|GetDistanceLocation (Variables|Temp|GetLastTraceLocation) (Transformation|GetActorLocation)))
        (Variables|Temp|SetLastTraceLocation (Transformation|GetActorLocation)))
      (if (Variables|Projectile|GetHoming)
        (if (Utilities|IsValid _target)
          (if (Variables|/Game/RPGSystem/Blueprints/BPC_RPGSystem.BPC_RPGSystem_C|GetIsDead _target)
            (if (Variables|Projectile|GetAllowNewSearch) :!label _label
              (CallFunction|GetTarget true))
            (else
              (Transformation|SetActorRotation (Math|Interpolation|Ease "EaseIn" 0.9 (Transformation|GetActorRotation) (Math|Rotator|FindLookatRotation _returnvalue_3 _returnvalue_6) true (+ (* (Math|Float|Max(Float) (/ (Math|Vector|VectorLength (- _returnvalue_3 _returnvalue_6)) (Variables|Projectile|GetHomingRange)) 0.0) 2e+01) 5.0)))))
          (else
            (goto _label)))
        (Utilities|IsValid _projectilemovement
          (:Is%20Valid
            (Variables|/Script/Engine.MovementComponent|SetVelocity _projectilemovement (Class|KismetMathLibrary|CreateVectorfromYawPitch _yaw _pitch (Variables|Projectile|GetSpeed)))))))))

(event EventBeginPlay
  (bind _projectilemovement (Variables|Default|GetProjectileMovement))
  ;[1 1 1] Begin
  (|CallParentFunction)
  (bind _output_get (Variables|Temp|SetStartLocation (Transformation|GetActorLocation)))
  (Variables|Temp|SetLastTraceLocation _output_get)
  (Utilities|IsValid _projectilemovement
    (:Is%20Valid
      (Variables|/Script/Engine.MovementComponent|SetVelocity _projectilemovement (Class|KismetMathLibrary|CreateVectorfromYawPitch (.yaw (Transformation|GetActorRotation)) 0.0 (Variables|Projectile|GetSpeed))))
    (:Is%20Not%20Valid
      _))
  (Actor|Tick|SetActorTickEnabled true))

(fn ConstructionScript
  (|CallParentFunction)
  (Variables|Projectile|SetSpeed (.ProjectileSpeed (Utilities|Struct|BreakS_Skill (Variables|Default|GetSkillInfo))))
  (Variables|/Script/Engine.ProjectileMovementComponent|SetMaxSpeed (Variables|Default|GetProjectileMovement) (Variables|Projectile|GetSpeed)))

(fn GetTarget
  (params (RandomTarget :type Boolean))
  (bind _returnvalue (Transformation|GetActorLocation))
  (bind _array (Utilities|Array|MakeArray "ObjectTypeQuery3"))
  (bind _varenemylist (LocalVariables|GetVarEnemyList))
  (bind _skillowner (Variables|Default|GetSkillOwner))
  (bind _homingrange (Variables|Projectile|GetHomingRange))
  (bind _returnvalue_2 (Utilities|Array|Length _varenemylist))
  (bind _returnvalue_3 (Components|GetOwner _skillowner))
  (bind _returnvalue_4 (- _returnvalue_2 1))
  (bind _array_2 (Utilities|Array|MakeArray _returnvalue_3))
  (bind _returnvalue_5 (select RandomTarget _returnvalue_4 0))
  (bind _returnvalue_6 (Math|Random|RandomIntegerinRange 0 _returnvalue_5))
  (bind _output (Utilities|Array|Get(acopy) _varenemylist _returnvalue_6))
  (Networking|SwitchHasAuthority
    (:Authority
      (switch Utilities|FlowControl|Switch|SwitchonE_SkillTraceType (Variables|Projectile|GetHomingTraceType)
        (:NewEnumerator0
          (bind _outhits (Collision|MultiSphereTraceForObjects _returnvalue _returnvalue (Variables|Projectile|GetHomingRange) _array false _array_2 "None"))
          (LocalVariables|SetVarHits _outhits))
        (:NewEnumerator1
          (bind _outhits_2 (Class|KismetSystemLibrary|BoxTraceMultiforObjects (Transformation|GetActorLocation) (+ (Variables|Temp|GetStartLocation) (* (Transformation|GetActorForwardVector) (Variables|Default|GetPlayerAttackDistanceUnits))) (Math|Vector|MakeVector 0.0 _homingrange _homingrange) (Transformation|GetActorRotation) _array false _array_2 "None" true))
          (LocalVariables|SetVarHits _outhits_2)))
      (bind _array_element (Utilities|Array|ForEachLoopwithBreak (LocalVariables|GetVarHits))
        (:LoopBody
          (if (.Valid (CallFunction|IsValidTarget (Variables|Default|GetSkillOwner) (.HitActor (Collision|BreakHitResult _array_element))))
            (if (.Return (Utilities|IsTargetinAngle (- (Transformation|GetActorLocation) (Transformation|GetActorLocation (Components|GetOwner (.Target%20 (CallFunction|IsValidTarget (Variables|Default|GetSkillOwner) (.HitActor (Collision|BreakHitResult _array_element))))))) (Variables|Projectile|GetHomingAngle) 1.8e+02 (Math|Vector|GetForwardVector (Transformation|GetActorRotation))))
              (Utilities|Array|Add (LocalVariables|GetVarEnemyList) (.Target%20 (CallFunction|IsValidTarget (Variables|Default|GetSkillOwner) (.HitActor (Collision|BreakHitResult _array_element))))))))
        (:Completed
          (if (> _returnvalue_2 0)
            (Utilities|IsValid _output
              (:Is%20Valid
                (Variables|Default|SetTarget _output)
                (Variables|Temp|SetTimeTarget (Utilities|Time|GetTimeSeconds)))
              (:Is%20Not%20Valid
                (Variables|Default|SetTarget 0 :!label _label)
                (Variables|Temp|SetTimeTarget 0.0)))
            (else
              (goto _label))))))))

(fn CollisionTrace
  (params (Start :type Vector) (Radius :type Float%20%28double-precision%29))
  (bind _collisionradius (Variables|Projectile|GetCollisionRadius))
  (if (not (Variables|Default|GetTriggered))
    (bind _outhits (Class|KismetSystemLibrary|BoxTraceMultiforObjects Start (+ Start (* (Transformation|GetActorForwardVector) Radius)) (Math|Vector|MakeVector 0.0 (.y _collisionradius) (.y _collisionradius)) (Transformation|GetActorRotation) (Utilities|Array|MakeArray "ObjectTypeQuery1" "ObjectTypeQuery2" "ObjectTypeQuery3") false (Utilities|Array|MakeArray (Components|GetOwner (Variables|Default|GetSkillOwner))) (Variables|Default|GetDrawDebugType) true))
    (bind _array_element (Utilities|Array|ForEachLoopwithBreak _outhits :!label _label)
      (:LoopBody
        (if (.Valid (CallFunction|IsValidTarget (Variables|Default|GetSkillOwner) (.HitActor (Collision|BreakHitResult _array_element))))
          (if (!= (.Target%20 (CallFunction|IsValidTarget (Variables|Default|GetSkillOwner) (.HitActor (Collision|BreakHitResult _array_element)))) (Variables|Default|GetSkillOwner))
            (CallFunction|OnCollided (.Target%20 (CallFunction|IsValidTarget (Variables|Default|GetSkillOwner) (.HitActor (Collision|BreakHitResult _array_element)))))
            (goto _label Break))
          (elif (.bSuccess (Utilities|Casting|CastToCharacter (.HitActor (Collision|BreakHitResult _array_element))))
            (goto _label Break)
            (else
              (CallFunction|OnCollided)
              (goto _label Break))))))))