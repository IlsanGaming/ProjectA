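; Swordsman Punch skill that chains dash attacks between random nearby targets, with damage and hit count scaled by skill level.
; Each hit shuffles a sphere trace, picks a valid RPG-system target and randomly aims in front of or behind it.
; A timeline dashes and turns the owner, then a DoOnce-gated AoE hit triggers the next search.
; Running out of hits or targets resets time dilation and ends the skill.
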(event Custom|StartNewAttack
  (bind _skillowner (Variables|Default|GetSkillOwner))
  (bind _hitcount (Variables|Default|GetHitCount))
  (bind _returnvalue (Components|GetOwner _skillowner))
  (bind _returnvalue_2 (Transformation|GetActorLocation _returnvalue))
  ;[1 1 1] Start new Attack
  (Math|Integer|DecrementInt _hitcount
    (:%20%20
      (if (> _hitcount 0)
        (bind _outhits (Collision|MultiSphereTraceForObjects _returnvalue_2 _returnvalue_2 8e+02 (Utilities|Array|MakeArray "ObjectTypeQuery3") false (Utilities|Array|MakeArray _returnvalue) "None" true "(R=1.000000,G=0.000000,B=0.000000,A=1.000000)" "(R=0.000000,G=1.000000,B=0.000000,A=1.000000)" 1.0))
        (Utilities|Array|Shuffle _outhits)
        (bind _array_element (Utilities|Array|ForEachLoopwithBreak _outhits :!label _label)
          (:LoopBody
            (bind (_success _reference) (Class|BPIRPGSystem|GetRPGSystem(Message) (.HitActor (Collision|BreakHitResult _array_element))))
            (if _success
              (bind _radius (Class|BPIRPGSystem|GetMeshRadius(Message) (.HitActor (Collision|BreakHitResult _array_element))))
              (if (Utilities|IsValid _reference)
                (if (.Valid (CallFunction|IsValidTarget (Variables|Default|GetSkillOwner) (.HitActor (Collision|BreakHitResult _array_element))))
                  (Variables|Default|SetTargetLocation (+ (Transformation|GetActorLocation (Components|GetOwner _reference)) (* (Transformation|GetActorForwardVector (Components|GetOwner _reference)) (Math|Float|SelectFloat (* (+ _radius 5e+01) -1.0) (+ _radius 5e+01) (Math|Random|RandomBoolwithWeight 0.5)))))
                  (Variables|Default|SetRotationPoint (Transformation|GetActorLocation (Components|GetOwner _reference)))
                  (Variables|Default|Setfound true)
                  (goto _label Break)))))
          (:Completed
            ;[1 1 1] Start Dash if found
            (if (Variables|Default|Getfound)
              (Variables|Default|Setfound false)
              (CallFunction|StartDash)
              (else
                (CallFunction|CancelSkill)))))
        (else
          (CallFunction|CancelSkill))))))

(event Custom|CancelSkill
  ;[1 1 1] Cancel
  (Default|SetCustomTimeDilationServer (Variables|Default|GetSkillOwner) 1.0)
  (Class|BPIRPGSystem|StopMovementInterface(Message) (Components|GetOwner (Variables|Default|GetSkillOwner)))
  (CallFunction|SkillEnd))

(event Custom|StartDash
  (bind _returnvalue (Transformation|GetActorRotation))
  (bind _skillowner (Variables|Default|GetSkillOwner))
  (bind _rotationpoint (Variables|Default|GetRotationPoint))
  (bind _skillowner_2 (Variables|Default|GetSkillOwner))
  (bind _skillowner_3 (Variables|Default|GetSkillOwner))
  (bind _targetlocation (Variables|Default|GetTargetLocation))
  (bind (_roll _pitch) (Math|Rotator|BreakRotator _returnvalue))
  (bind _returnvalue_2 (Components|GetOwner _skillowner_3))
  (bind _returnvalue_3 (Components|GetOwner _skillowner_2))
  (bind _returnvalue_4 (Components|GetOwner _skillowner))
  (bind _returnvalue_5 (Transformation|GetActorLocation _returnvalue_3))
  (bind _returnvalue_6 (Transformation|GetActorLocation _returnvalue_4))
  (bind _returnvalue_7 (- _targetlocation _returnvalue_5))
  (bind _returnvalue_8 (Math|Rotator|FindLookatRotation _returnvalue_6 _rotationpoint))
  (bind _yaw (Math|Rotator|BreakRotator _returnvalue_8))
  (bind _returnvalue_9 (Math|Rotator|MakeRotator _roll _pitch _yaw))
  ;[1 1 1] 'Dash' to target and set rotation
  (bind _newtrack_1 (Timeline|Timeline_0 PlayFromStart)
    (:Update
      (Transformation|SetActorLocation _returnvalue_2 (Math|Vector|Lerp(Vector) _returnvalue_5 (+ _returnvalue_5 (* _returnvalue_7 _newtrack_1)) 0.9) false true)
      (Transformation|SetActorRotation _returnvalue_2 _returnvalue_9 true)
      (Class|BPIRPGSystem|SetRotationfromServer(Message) _returnvalue_3 _returnvalue_9 true)
      (if (< (Math|Vector|VectorLength _returnvalue_7) 5e+01)
        (Utilities|FlowControl|Sequence
          (:then_0
            (Timeline|Timeline_0 Stop))
          (:then_1
            (Utilities|FlowControl|DoOnce false :!label _label
              (:Completed
                (CallFunction|DoDamageAoe)
                (CallFunction|StartNewAttack)))))))
    (:Finished
      (goto _label))))

(event EventHitAoe
  (bind _skillowner (Variables|Default|GetSkillOwner))
  (bind _skillinfo (Variables|Default|GetSkillInfo))
  (bind _skilllevel (Variables|Default|GetSkillLevel))
  (bind (_damagepercent _multihitcount) (Utilities|Struct|BreakS_Skill _skillinfo))
  (bind _returnvalue (Components|GetOwner _skillowner))
  (bind _returnvalue_2 (Transformation|GetActorLocation _returnvalue))
  (Variables|Default|SetStartTransform (Transformation|GetActorTransform _returnvalue))
  (Class|BPIRPGSystem|StopMovementInterface(Message) _returnvalue)
  (Utilities|Struct|SetmembersinS_Skill _skillinfo (+ (* _skilllevel 1e+01) _damagepercent) (+ _skilllevel _multihitcount))
  (CallFunction|SetMultiHitInfo)
  (bind _outhits (Collision|MultiSphereTraceForObjects _returnvalue_2 _returnvalue_2 8e+02 (Utilities|Array|MakeArray "ObjectTypeQuery3") false (Utilities|Array|MakeArray _returnvalue) "None" true "(R=1.000000,G=0.000000,B=0.000000,A=1.000000)" "(R=0.000000,G=1.000000,B=0.000000,A=1.000000)" 1.0))
  (Utilities|Array|Shuffle _outhits)
  (bind _array_element (Utilities|Array|ForEachLoopwithBreak _outhits :!label _label)
    (:LoopBody
      (bind (_success _reference) (Class|BPIRPGSystem|GetRPGSystem(Message) (.HitActor (Collision|BreakHitResult _array_element))))
      (if _success
        (bind _radius (Class|BPIRPGSystem|GetMeshRadius(Message) (.HitActor (Collision|BreakHitResult _array_element))))
        (if (Utilities|IsValid _reference)
          (if (.Valid (CallFunction|IsValidTarget (Variables|Default|GetSkillOwner) (.HitActor (Collision|BreakHitResult _array_element))))
            (Variables|Default|SetTargetLocation (+ (Transformation|GetActorLocation (Components|GetOwner _reference)) (* (Transformation|GetActorForwardVector (Components|GetOwner _reference)) (Math|Float|SelectFloat (* (+ _radius 5e+01) -1.0) (+ _radius 5e+01) (Math|Random|RandomBoolwithWeight 0.5)))))
            (Variables|Default|SetRotationPoint (Transformation|GetActorLocation (Components|GetOwner _reference)))
            (Variables|Default|Setfound true)
            (goto _label Break)))))
    (:Completed
      ;[1 1 1] Start Dash if found
      (if (Variables|Default|Getfound)
        (Variables|Default|Setfound false)
        (CallFunction|StartDash)
        (else
          (CallFunction|CancelSkill))))))

(event EventOnHit
  (params (Target :type BPC%20RPG%20System%20Object%20Reference))
  ;[1 1 1] Comment
  (Class|BPIRPGSystem|DoCameraShake(Message) (Components|GetOwner (Variables|Default|GetSkillOwner)) "/Game/RPGSystem/Blueprints/CameraShakes/CS_ExampleShake.CS_ExampleShake_C" (Transformation|GetActorLocation) 0.0 2.5e+03 0.05 false))

(event EventOnAoeHitDone
  (params (Targets :type Array%20of%20BPC%20RPG%20System%20Object%20References))
  ;[1 1 1] 'Dash' to target and set rotation
  (Utilities|FlowControl|DoOnce false) ; enters at Reset
)

(fn ConstructionScript
  (|CallParentFunction))