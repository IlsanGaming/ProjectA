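; Swordman Bowling Bash skill Blueprint that computes its damage when the skill starts and then applies the hit.
; Damage is a random roll between the owner's min and max ATK as a percentage, multiplied by four times the base damage plus a per-level bonus.
; It writes that value into SkillInfo, then branches on the SingleTarget flag to call either the single-target or area-of-effect hit function.
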(event EventBeginPlay)

(event Collision|EventActorBeginOverlap
  (params (OtherActor :type Actor%20Object%20Reference)))

(event EventTick
  (params (DeltaSeconds :type Float%20%28single-precision%29)))

(event EventSkillStart
  (bind _skillinfo (Variables|Default|GetSkillInfo))
  (bind _skillowner (Variables|Default|GetSkillOwner))
  (bind (_attacktype _damage _singletarget) (Utilities|Struct|BreakS_Skill _skillinfo))
  (bind _playerinfo (Variables|/Game/RPGSystem/Blueprints/BPC_RPGSystem.BPC_RPGSystem_C|GetPlayerInfo _skillowner))
  (bind _stats (Utilities|Struct|BreakS_PlayerInfo _playerinfo))
  (bind (_minatk _maxatk) (Utilities|Struct|BreakS_Stats _stats))
  (Utilities|Struct|SetmembersinS_Skill _skillinfo (* (/ (Math|Conversions|ToFloat(Integer) (Math|Random|RandomIntegerinRange _minatk _maxatk)) 1e+02) (* (+ _damage (Math|Conversions|ToFloat(Integer) (* (Variables|Default|GetSkillLevel) 40))) 4.0)))
  (if _singletarget
    (CallFunction|HitSingleTarget)
    (else
      (CallFunction|HitAoe))))

(fn ConstructionScript
  (|CallParentFunction))