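; Swordman Earth Strike skill: an advancing, widening ground attack of three staged blasts in front of the actor.
; On authority it detaches, then fires waves at short delays and ends the skill after the last.
; Each wave spawns a BP_Skill_Boom with a farther, wider box trace, plus a growing row of lowered fire-impact particles.
; Blast damage scales from the skill's base, much lower when the owner's PlayerAI flag is set.
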(event Custom|SpawnBomb
  (params (Spawn%20Transform%20Location :type Vector) (BoxTraceSettings :type S%20Skill%20Box%20Trace%20Settings%20Structure))
  ;[1 1 1] Comment
  (Utilities|Struct|SetmembersinS_Skill (Variables|Default|GetCustomSkillInfo) (* (.Damage (Utilities|Struct|BreakS_Skill (Variables|Default|GetSkillInfo))) (Math|Float|SelectFloat 0.25 1.5 (Variables|/Game/RPGSystem/Blueprints/BPC_RPGSystem.BPC_RPGSystem_C|GetPlayerAI (Variables|Default|GetSkillOwner)))) "NewEnumerator1" BoxTraceSettings)
  (Game|SpawnActorfromClass "/Game/RPGSystem/Blueprints/Skill/Swordman/BP_Skill_Boom.BP_Skill_Boom_C" (Math|Transform|MakeTransform Spawn%20Transform%20Location (Transformation|GetActorRotation) "1.000000,1.000000,1.000000") "AlwaysSpawn" "OverrideRootScale" self (Variables|Default|GetCustomSkillInfo) (Variables|Default|GetSkillOwner) 1 "None" 0 (Variables|Default|GetKey) 0))

(event Custom|SpawnParticle
  (params (Location :type Vector))
  (Class|BPIRPGSystem|GetMeshRadius(Message) (Variables|Default|GetSkillOwner))
  ;[1 1 1] Comment
  (CallFunction|SpawnParticles "/Game/RPGSystem/Particles/P_Impact_Enemy_Gib_Fire.P_Impact_Enemy_Gib_Fire" "0, 0, 0" (- (Transformation|GetActorLocation) (Math|Vector|MakeVector 0.0 0.0 1.7e+02)) Location "1.000000,1.000000,1.000000" 0.0 false))

(event EventSkillStart
  (bind _returnvalue (Transformation|GetActorRotation))
  (bind _returnvalue_2 (Transformation|GetActorLocation))
  (bind _returnvalue_3 (Math|Vector|GetRightVector _returnvalue))
  (bind _returnvalue_4 (Math|Vector|GetForwardVector _returnvalue))
  (bind _returnvalue_5 (* _returnvalue_4 1.8e+02))
  (bind _returnvalue_6 (* _returnvalue_4 3e+02))
  ;[1 1 1] Comment
  (Networking|SwitchHasAuthority
    (:Authority
      (Transformation|DetachFromActor "KeepWorld" "KeepWorld" "KeepWorld")
      (CallFunction|SpawnBomb _returnvalue_2 (Utilities|Struct|MakeS_SkillBoxTraceSettings 1e+01 1e+02 6e+01 0.0))
      (CallFunction|SpawnParticle (* _returnvalue_4 6e+01))
      (Utilities|FlowControl|Delay 0.2)
      (CallFunction|SpawnBomb _returnvalue_2 (Utilities|Struct|MakeS_SkillBoxTraceSettings 1.3e+02 1e+02 1.1e+02 0.0))
      (CallFunction|SpawnParticle (+ "0, 0, 0" _returnvalue_5 (* _returnvalue_3 -55.0)))
      (CallFunction|SpawnParticle (+ "0, 0, 0" _returnvalue_5 (* _returnvalue_3 55.0)))
      (Utilities|FlowControl|Delay 0.2)
      (CallFunction|SpawnBomb _returnvalue_2 (Utilities|Struct|MakeS_SkillBoxTraceSettings 2.5e+02 1e+02 1.6e+02 0.0))
      (CallFunction|SpawnParticle (+ "0, 0, 0" _returnvalue_6 (* _returnvalue_3 1.1e+02)))
      (CallFunction|SpawnParticle (+ "0, 0, 0" _returnvalue_6 (* _returnvalue_3 -1.1e+02)))
      (CallFunction|SpawnParticle (+ "0, 0, 0" _returnvalue_6))
      (CallFunction|SkillEnd))))

(fn ConstructionScript
  (|CallParentFunction))