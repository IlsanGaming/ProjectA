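; Base shop NPC for the RPG system that lets the player open and close a shop through interaction.
; Interact toggles the NPC's BPCShop component through RPGSystem, closing any current shop or opening this one.
; Tooltip-triggered interactions first require a horizontal distance check against MinDistanceToTalk plus a margin, while other commands skip it.
; Getter functions supply the shop component, move destination, open/close screen prompt and shop-name world label.
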(event EventInteract
  (params (RPGSystem :type BPC%20RPG%20System%20Object%20Reference) (Command :type String))
  ;[1 1 1] Interact
  (if (Utilities|Enum|Equal(Enum) Command "FromTooltip")
    (bind _action (CallFunction|GetInteractInfo RPGSystem))
    (if (Utilities|Enum|Equal(Enum) _action "NewEnumerator0")
      (Utilities|IsValid (Variables|/Game/RPGSystem/Blueprints/BPC_RPGSystem.BPC_RPGSystem_C|GetCurrentShop RPGSystem) :!label _label
        (:Is%20Valid
          (Default|CloseShop RPGSystem))
        (:Is%20Not%20Valid
          (Default|OpenShop RPGSystem (Variables|Default|GetBPC_Shop)))))
    (else
      (goto _label))))

(fn ConstructionScript)

(fn GetInteractInfo
  (params (RPGSystem :type BPC%20RPG%20System%20Object%20Reference))
  (bind _worldlocation (CallFunction|GetMovetoEndDestination))
  (return true (select (< (- (CallFunction|GetDistanceXY (Transformation|GetActorLocation (Components|GetOwner RPGSystem)) _worldlocation) (Variables|Default|GetMinDistanceToTalk)) 2.5e+02) "NewEnumerator0" "NewEnumerator1")))

(fn GetMovetoEndDestination
  (return true (Transformation|GetActorLocation)))

(fn GetScreenTooltipInfo
  (params (RPGSystem :type BPC%20RPG%20System%20Object%20Reference))
  (return true (select (Utilities|IsValid (Variables|/Game/RPGSystem/Blueprints/BPC_RPGSystem.BPC_RPGSystem_C|GetCurrentShop RPGSystem)) "Close Shop [E]" "Open Shop [E]") "(R=1.000000,G=1.000000,B=1.000000,A=1.000000)"))

(fn GetShopComponent
  (return true (Variables|Default|GetBPC_Shop)))

(fn GetWorldTooltipInfo
  (return true false (Utilities|Struct|BreakS_Shop (Variables|/Game/RPGSystem/Blueprints/BPC_Shop.BPC_Shop_C|GetShopInfo (Variables|Default|GetBPC_Shop))) "(R=1.000000,G=1.000000,B=1.000000,A=1.000000)" "0, 0,105.000000"))