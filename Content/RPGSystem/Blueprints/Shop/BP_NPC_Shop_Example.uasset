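; Example shop NPC Blueprint for the RPG System that extends an inherited interactable NPC.
; On BeginPlay it adds the skeletal mesh's bounding sphere radius to the talk distance, and selection toggles custom depth on the mesh for an outline.
; Interact passes straight to the parent.
; An unconnected example shows a server-side custom variable message for updating a quest task when the shop is used.
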(event EventBeginPlay
  ;[1 1 1] Add Skeletal Mesh Radius to InteractRange
  (|CallParentFunction)
  (Variables|Default|SetMinDistanceToTalk (+ (Variables|Default|GetMinDistanceToTalk) (.SphereRadius (Collision|GetComponentBounds (Variables|Default|GetSkeletalMesh))))))

(event EventInteract
  (params (RPGSystem :type BPC%20RPG%20System%20Object%20Reference) (Command :type String))
  (|CallParentFunction RPGSystem Command))

(event EventSelectInteractable
  (params (Selected :type Boolean))
  ;[1 1 1] Outline
  (Rendering|SetRenderCustomDepth (Variables|Default|GetSkeletalMesh) Selected))

(fn ConstructionScript
  (|CallParentFunction))