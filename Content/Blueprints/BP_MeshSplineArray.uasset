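; Construction-script tool that places copies of a chosen mesh at a set spacing along a spline as Hierarchical Instanced Static Mesh instances.
; Each instance faces the spline tangent, then applies a base transform, with location offsets added in world space.
; One seeded stream value between -1 and 1 per instance scales the location, rotation and scale randomness together, so those variations are correlated.
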(event EventBeginPlay)

(event Collision|EventActorBeginOverlap
  (params (OtherActor :type Actor%20Object%20Reference)))

(event EventTick
  (params (DeltaSeconds :type Float%20%28single-precision%29)))

(fn ConstructionScript
  (bind _spline (Variables|Default|GetSpline))
  (bind _base_instance_transform (Variables|Default|GetBase%20Instance%20Transform))
  (bind _transform_randomness (Variables|Default|GetTransform%20Randomness))
  (bind _mesh (Variables|Default|GetMesh)
    (:then
      (Components|StaticMesh|SetStaticMesh (Variables|Default|GetHierarchicalInstancedStaticMesh) _mesh)
      (while (<= (LocalVariables|GetNextDistance) (Spline|GetSplineLength (Variables|Default|GetSpline)))
        (LocalVariables|SetRandomStreamNumber (Math|Random|RandomFloatinRangefromStream (Variables|Default|GetRandomStream) -1.0 1.0))
        (Class|InstancedStaticMeshComponent|AddInstanceWorldSpace (Variables|Default|GetHierarchicalInstancedStaticMesh) (Math|Transform|MakeTransform (+ (Spline|GetLocationatDistanceAlongSpline _spline (LocalVariables|GetNextDistance) "World") (.location _base_instance_transform) (* (.location _transform_randomness) (LocalVariables|GetRandomStreamNumber))) (Math|Rotator|CombineRotators (Math|Rotator|CombineRotators (Math|Conversions|RotationFromXVector (Spline|GetTangentatDistanceAlongSpline _spline (LocalVariables|GetNextDistance) "World")) (.rotation _base_instance_transform)) (* (.rotation _transform_randomness) (LocalVariables|GetRandomStreamNumber))) (+ (.scale _base_instance_transform) (* (.scale _transform_randomness) (LocalVariables|GetRandomStreamNumber)))))
        (LocalVariables|SetNextDistance (+ (LocalVariables|GetNextDistance) (Variables|Default|GetSpacing)))))
    (:else)))