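; An elevator that a player standing in its trigger box operates with the F key, with a widget shown while in range.
; F plays a sound and, by a toggle, runs one of two timeline sets at TimeRate to move the cube vertically, scaled by MoveLength.
; Parallel timelines rescale the wire to match, branching on the sign of MoveLength.
; The construction script sets the wire's initial length from MoveLength and WireBorder.
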(event OnComponentBeginOverlap(Box)
  (params (OverlappedComponent :type Primitive%20Component%20Object%20Reference) (OtherActor :type Actor%20Object%20Reference) (OtherComp :type Primitive%20Component%20Object%20Reference) (OtherBodyIndex :type Integer) (bFromSweep :type Boolean) (SweepResult :type Hit%20Result%20Structure%20%28by%20ref%29))
  (Input|EnableInput (Game|GetPlayerController 0))
  (Rendering|SetVisibility (Variables|Default|GetWidget) true false))

(event OnComponentEndOverlap(Box)
  (params (OverlappedComponent :type Primitive%20Component%20Object%20Reference) (OtherActor :type Actor%20Object%20Reference) (OtherComp :type Primitive%20Component%20Object%20Reference) (OtherBodyIndex :type Integer))
  (Input|DisableInput (Game|GetPlayerController 0))
  (Rendering|SetVisibility (Variables|Default|GetWidget) false false))

(event Input|KeyboardEvents|F
  (params (Key :type Key%20Structure))
  (bind _movelength (Variables|Default|GetMoveLength))
  (bind _movelength_2 (Variables|Default|GetMoveLength))
  (bind _movelength_3 (Variables|Default|GetMoveLength))
  (bind _wire (Variables|Default|GetWire))
  (bind _movelength_4 (Variables|Default|GetMoveLength))
  (bind _wire_2 (Variables|Default|GetWire))
  (bind _returnvalue (* _movelength -1.0))
  (bind _returnvalue_2 (* _movelength_4 -1.0))
  (:Pressed
    (Audio|PlaySound2D "/Game/Sounds/Elevator_01.Elevator_01" 1.0 1.0 0.0 0 0)
    (Rendering|SetVisibility (Variables|Default|GetWidget) false false)
    (Components|Timeline|SetPlayRate (Variables|Default|GetTimeline) (Variables|Default|GetTimeRate))
    (if (Variables|Default|GetToggleSwitch)
      (Utilities|FlowControl|Sequence
        (:then_0
          (bind _newtrack_0 (Timeline|Timeline Play)
            (:Update
              (Transformation|SetRelativeLocation (Variables|Default|GetCube) (* _newtrack_0 (Math|Vector|MakeVector 0.0 0.0 (Variables|Default|GetMoveLength))) false false)
              (Variables|Default|SetToggleSwitch false))))
        (:then_1
          (if (> (Variables|Default|GetMoveLength) 0.0)
            (bind _newtrack_0_2 (Timeline|Timeline_0 Play)
              (:Update
                (Transformation|SetRelativeScale3D (Variables|Default|GetWire) (Math|Vector|MakeVector 0.1 0.1 (- (+ _movelength_3 (Variables|Default|GetWireBorder)) (* _movelength_3 _newtrack_0_2))))))
            (else
              (bind _newtrack_0_3 (Timeline|Timeline_1 Play)
                (:Update
                  (Transformation|SetRelativeScale3D _wire (Math|Vector|MakeVector 0.1 0.1 (+ (Variables|Default|GetWireBorder) (* _returnvalue_2 _newtrack_0_3)))))
                (:Finished
                  (Transformation|SetRelativeScale3D _wire (Math|Vector|MakeVector 0.1 0.1 _returnvalue_2))))))))
      (else
        (Utilities|FlowControl|Sequence
          (:then_0
            (bind _newtrack_0_4 (Timeline|Timeline_2 Play)
              (:Update
                (Transformation|SetRelativeLocation (Variables|Default|GetCube) (* _newtrack_0_4 (Math|Vector|MakeVector 0.0 0.0 (Variables|Default|GetMoveLength))) false false)
                (Variables|Default|SetToggleSwitch true))))
          (:then_1
            (if (> (Variables|Default|GetMoveLength) 0.0)
              (bind _newtrack_0_5 (Timeline|Timeline_3 Play)
                (:Update
                  (Transformation|SetRelativeScale3D (Variables|Default|GetWire) (Math|Vector|MakeVector 0.1 0.1 (- (+ _movelength_2 (Variables|Default|GetWireBorder)) (* _movelength_2 _newtrack_0_5))))))
              (else
                (bind _newtrack_0_6 (Timeline|Timeline_4 Play)
                  (:Update
                    (Transformation|SetRelativeScale3D _wire_2 (Math|Vector|MakeVector 0.1 0.1 (+ (Variables|Default|GetWireBorder) (* _returnvalue _newtrack_0_6)))))
                  (:Finished
                    (Transformation|SetRelativeScale3D _wire_2 (Math|Vector|MakeVector 0.1 0.1 _returnvalue))))))))))))

(fn ConstructionScript
  (bind _wire (Variables|Default|GetWire))
  (bind _movelength (Variables|Default|GetMoveLength))
  (bind _wireborder (Variables|Default|GetWireBorder))
  (if (> _movelength 0.0)
    (Transformation|SetRelativeScale3D _wire (Math|Vector|MakeVector 0.1 0.1 (+ _movelength _wireborder)))
    (else
      (Transformation|SetRelativeScale3D _wire (Math|Vector|MakeVector 0.1 0.1 _wireborder)))))