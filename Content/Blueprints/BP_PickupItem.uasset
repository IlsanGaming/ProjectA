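; BP_PickupItem is a pickup actor with a configurable mesh, assigned in the construction script from PickupMesh.
; Box overlap enables input for player 0 and shows a widget, without filtering the overlapping actor; leaving reverses both.
; Pressing F hides the item and widget, disables collision, stops the glow, plays a sound and Niagara effect, then destroys the actor after a delay.
; No item is granted to the player here.
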(event OnComponentBeginOverlap(Box)
  (params (OverlappedComponent :type Primitive%20Component%20Object%20Reference) (OtherActor :type Actor%20Object%20Reference) (OtherComp :type Primitive%20Component%20Object%20Reference) (OtherBodyIndex :type Integer) (bFromSweep :type Boolean) (SweepResult :type Hit%20Result%20Structure%20%28by%20ref%29))
  (Input|EnableInput (Game|GetPlayerController 0))
  (Rendering|SetVisibility (Variables|Default|GetWidget) true false))

(event OnComponentEndOverlap(Box)
  (params (OverlappedComponent :type Primitive%20Component%20Object%20Reference) (OtherActor :type Actor%20Object%20Reference) (OtherComp :type Primitive%20Component%20Object%20Reference) (OtherBodyIndex :type Integer))
  (Input|DisableInput (Game|GetPlayerController 0))
  (Rendering|SetVisibility (Variables|Default|GetWidget) false false))

(event Input|KeyboardEvents|F
  (params (Key :type Key%20Structure))
  (bind _pickupitem (Variables|Default|GetPickupItem))
  (:Pressed
    (Rendering|SetVisibility (Variables|Default|GetWidget) false false)
    (Development|SetHiddeninGame _pickupitem true false)
    (Collision|SetCollisionEnabled _pickupitem "NoCollision")
    (Components|Activation|Deactivate (Variables|Default|GetGlow))
    (Audio|PlaySound2D 0 1.0 1.0 0.0 0 0)
    (Components|Activation|Activate (Variables|Default|GetNiagara) false)
    (Utilities|FlowControl|Delay 5.0)
    (Actor|DestroyActor)))

(fn ConstructionScript
  (Components|StaticMesh|SetStaticMesh (Variables|Default|GetPickupItem) (Variables|Default|GetPickupMesh)))