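; BP_Door_Double_02 is an interactive double door that the player opens by pressing F nearby.
; Box overlap begin and end toggle player 0 input and a prompt widget, without filtering the overlapping actor.
; F plays a 2D sound, hides the prompt and plays two timelines that drive the yaw of DoorL and DoorR.
; The graph has no closing logic.
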(event OnComponentBeginOverlap(Box)
  (params (OverlappedComponent :type Primitive%20Component%20Object%20Reference) (OtherActor :type Actor%20Object%20Reference) (OtherComp :type Primitive%20Component%20Object%20Reference) (OtherBodyIndex :type Integer) (bFromSweep :type Boolean) (SweepResult :type Hit%20Result%20Structure%20%28by%20ref%29))
  (Input|EnableInput (Game|GetPlayerController 0))
  (Rendering|SetVisibility (Variables|Default|GetWidget) true false))

(event OnComponentEndOverlap(Box)
  (params (OverlappedComponent :type Primitive%20Component%20Object%20Reference) (OtherActor :type Actor%20Object%20Reference) (OtherComp :type Primitive%20Component%20Object%20Reference) (OtherBodyIndex :type Integer))
  (Input|DisableInput (Game|GetPlayerController 0))
  (Rendering|SetVisibility (Variables|Default|GetWidget) false false))

(event Input|KeyboardEvents|F
  (params (Key :type Key%20Structure))
  (:Pressed
    (Audio|PlaySound2D "/Game/Sounds/DoorOpen_01.DoorOpen_01" 1.0 1.0 0.0 0 0)
    (Rendering|SetVisibility (Variables|Default|GetWidget) false false)
    (Utilities|FlowControl|Sequence
      (:then_0
        (bind _newtrack_0 (Timeline|Timeline Play)
          (:Update
            (Transformation|SetRelativeRotation (Variables|Default|GetDoor_L) (Math|Rotator|MakeRotator 0.0 0.0 (.z _newtrack_0)) false false))))
      (:then_1
        (bind _newtrack_0_2 (Timeline|Timeline_0 Play)
          (:Update
            (Transformation|SetRelativeRotation (Variables|Default|GetDoor_R) (Math|Rotator|MakeRotator 0.0 0.0 (.z _newtrack_0_2)) false false)))))))

(fn ConstructionScript)